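; Player character for a side-view platformer, with movement, jumping and interaction driven by Enhanced Input.
; BeginPlay adds the IMC_Platform mapping context, and jump input starts and stops the Character jump.
; Movement is locked to the world X axis, snapping control rotation yaw to face the input direction.
; Interact sends InteractMessage to the first overlapping actor that implements BP_InteractInterface.
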(event `self.ReceiveBeginPlay`
  (`|ExecutionSequence`
    (:`then_0`
      ;[1 1 1] Adding input mapping
      (bind _asplayer_controller (cast `PlayerController` (`self.GetController`)))
      (`EnhancedInputSubsystemInterface.AddMappingContext` (pcsubsystem `EnhancedInputLocalPlayerSubsystem` _asplayer_controller) "/Game/Inputs/IMC_Platform.IMC_Platform" 0 (struct)))))

(event `EnhancedInput|/Game/Inputs/Actions/IA_Jump`
  (params (ActionValue :type Boolean) (ElapsedSeconds :type "Float (double-precision)") (TriggeredSeconds :type "Float (double-precision)") (InputAction :type "InputAction Object Reference" :default "/Game/Inputs/Actions/IA_Jump.IA_Jump"))
  (:`Started`
    (`self.Jump`))
  (:`Completed`
    (`self.StopJumping`)))

(event `EnhancedInput|/Game/Inputs/Actions/IA_Move`
  (params (ActionValue :type "Float (double-precision)") (ElapsedSeconds :type "Float (double-precision)") (TriggeredSeconds :type "Float (double-precision)") (InputAction :type "InputAction Object Reference" :default "/Game/Inputs/Actions/IA_Move.IA_Move"))
  (:`Triggered`
    (`self.AddMovementInput` (1.0 0.0 0.0) ActionValue)
    (`Controller.SetControlRotation` (`self.GetController`) (select `bool` (> ActionValue 0.0) :`false` (`KismetMathLibrary.MakeRotator` 0.0 0.0 180.0) :`true` (`KismetMathLibrary.MakeRotator` 0.0)))))

(event `EnhancedInput|/Game/Inputs/Actions/IA_Interact`
  (params (ActionValue :type Boolean) (ElapsedSeconds :type "Float (double-precision)") (TriggeredSeconds :type "Float (double-precision)") (InputAction :type "InputAction Object Reference" :default "/Game/Inputs/Actions/IA_Interact.IA_Interact"))
  (:`Started`
    (for _array_element (`self.GetOverlappingActors` null)
      (if (`KismetSystemLibrary.DoesImplementInterface` _array_element "/Game/Blueprints/Platformer/BP_InteractInterface.BP_InteractInterface_C")
        (message `/Game/Blueprints/Platformer/BP_InteractInterface.Interact` _array_element)
        (break)))))

(fn `UserConstructionScript`)