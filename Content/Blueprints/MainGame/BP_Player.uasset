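; Player character for a top-down dungeon game, with mouse-aimed sphere-trace attacks, overlap-based interaction and an overlay widget.
; BPCCombat holds stats, restored from the game instance when saved, drives movement speed, and reports damage and death, which reloads MainArea.
; Warp events teleport the player and ease the camera across, likely between rooms, with brief invincibility.
; Debug keys adjust coins, masks and health, save currency, load MainArea or possess a debug pawn.
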(event `self.ReceiveBeginPlay`
  (bind _charactermovement (`self.CharacterMovement`))
  (bind (_stats_health _stats_maxhealth _stats_damage _stats_speed) (break `/Game/Blueprints/MainGame/Combat/ST_Stats` (`/Game/Blueprints/MainGame/Combat/BPC_Combat.Stats` (`self.BPC_Combat`))))
  (bind _stats_health_2 (break `/Game/Blueprints/MainGame/Combat/ST_Stats` (`/Game/Blueprints/MainGame/Combat/BPC_Combat.Stats` (`self.BPC_Combat`))))
  (`|ExecutionSequence`
    (:`then_0`
      ;[1 1 1] Add inputs
      (bind _asplayer_controller (cast `PlayerController` (`self.GetController`)))
      (`EnhancedInputSubsystemInterface.AddMappingContext` (pcsubsystem `EnhancedInputLocalPlayerSubsystem` _asplayer_controller) "/Game/Inputs/IMC_MainGame.IMC_MainGame" 0 (struct))
      (bind _returnvalue (`|CreateWidget` "/Game/Blueprints/MainGame/Widgets/W_PlayerOverlay.W_PlayerOverlay_C"))
      (bind _output_get (set `self.W_Overlay` _returnvalue))
      (`UserWidget.AddToViewport` _output_get 0)
      (set `PlayerController.bShowMouseCursor` true (`GameplayStatics.GetPlayerController` 0)))
    (:`then_1`
      ;[1 1 1] Stats
      (set `CharacterMovementComponent.MaxWalkSpeed` _stats_speed _charactermovement)
      (set `CharacterMovementComponent.MaxAcceleration` (* _stats_speed 3.5) _charactermovement)
      (`KismetSystemLibrary.PrintString` (`KismetStringLibrary.Concat_StrStr` "Health: " (`KismetStringLibrary.Conv_IntToString` _stats_health_2)) true true (struct :`R` 0.447917 :`B` 0.048566 :`A` 1.0) 5.0))))

(event `EnhancedInput|/Game/Inputs/Actions/IA_DungeonMove`
  (params (ActionValue :type "Vector2D Structure") (ElapsedSeconds :type "Float (double-precision)") (TriggeredSeconds :type "Float (double-precision)") (InputAction :type "InputAction Object Reference" :default "/Game/Inputs/Actions/IA_DungeonMove.IA_DungeonMove"))
  ;[1 1 1] Movement
  (:`Triggered`
    (if (`self.CanMove`)
      (`self.AddMovementInput` (0.0 -1.0 0.0) ActionValue_Y)
      (`self.AddMovementInput` (1.0 0.0 0.0) ActionValue_X))))

(event `WarpVertical`
  (params (Scale :type Integer))
  (bind _camera (`self.Camera`))
  (bind (_returnvalue_x _returnvalue_y _returnvalue_z) (`KismetMathLibrary.BreakVector` (`SceneComponent.K2_GetComponentLocation` (`self.Camera`))))
  (bind (_returnvalue_x_2 _returnvalue_y_2) (`KismetMathLibrary.BreakVector` (`SceneComponent.K2_GetComponentLocation` (`self.CapsuleComponent`))))
  ;[1 1 1] Warp Up/Down
  (set `/Game/Blueprints/MainGame/Combat/BPC_Combat.IsInvincible` true (`self.BPC_Combat`))
  (`SceneComponent.K2_SetWorldLocation` (`self.CapsuleComponent`) (`KismetMathLibrary.MakeVector` _returnvalue_x_2 (+ (* Scale 370) _returnvalue_y_2) 50.0) false false)
  (`KismetSystemLibrary.MoveComponentTo` _camera (`KismetMathLibrary.MakeVector` _returnvalue_x (+ (* 2050 Scale) _returnvalue_y) _returnvalue_z) (`SceneComponent.RelativeRotation` _camera) true true)
  (set `self.CanMove` false)
  (`KismetSystemLibrary.Delay` 0.05)
  (set `self.CanMove` true)
  (`KismetSystemLibrary.Delay` 1.0)
  (set `/Game/Blueprints/MainGame/Combat/BPC_Combat.IsInvincible` false (`self.BPC_Combat`)))

(event `WarpHorizontal`
  (params (Scale :type Integer))
  (bind _camera (`self.Camera`))
  (bind (_returnvalue_x _returnvalue_y _returnvalue_z) (`KismetMathLibrary.BreakVector` (`SceneComponent.K2_GetComponentLocation` (`self.Camera`))))
  (bind (_returnvalue_x_2 _returnvalue_y_2) (`KismetMathLibrary.BreakVector` (`SceneComponent.K2_GetComponentLocation` (`self.CapsuleComponent`))))
  ;[1 1 1] Warp Left/Right
  (set `/Game/Blueprints/MainGame/Combat/BPC_Combat.IsInvincible` true (`self.BPC_Combat`))
  (`SceneComponent.K2_SetWorldLocation` (`self.CapsuleComponent`) (`KismetMathLibrary.MakeVector` (+ (* Scale 350) _returnvalue_x_2) _returnvalue_y_2 50.0) false false)
  (`KismetSystemLibrary.MoveComponentTo` _camera (`KismetMathLibrary.MakeVector` (+ (* 2650 Scale) _returnvalue_x) _returnvalue_y _returnvalue_z) (`SceneComponent.RelativeRotation` _camera) true true)
  (set `self.CanMove` false)
  (`KismetSystemLibrary.Delay` 0.05)
  (set `self.CanMove` true)
  (`KismetSystemLibrary.Delay` 1.0)
  (set `/Game/Blueprints/MainGame/Combat/BPC_Combat.IsInvincible` false (`self.BPC_Combat`)))

(event `DamageResponse`
  (bind _bpc_combat (`self.BPC_Combat`))
  (bind _stats_health (break `/Game/Blueprints/MainGame/Combat/ST_Stats` (`/Game/Blueprints/MainGame/Combat/BPC_Combat.Stats` (`self.BPC_Combat`))))
  ;[1 1 1] Take Damage
  (`KismetSystemLibrary.PrintString` "Player Hit")
  (set `/Game/Blueprints/MainGame/Combat/BPC_Combat.IsInvincible` true _bpc_combat)
  (`KismetSystemLibrary.Delay` 1.0)
  (set `/Game/Blueprints/MainGame/Combat/BPC_Combat.IsInvincible` false _bpc_combat)
  (`KismetSystemLibrary.PrintString` (`KismetStringLibrary.Concat_StrStr` "Health: " (`KismetStringLibrary.Conv_IntToString` _stats_health)) true true (struct :`R` 0.447917 :`B` 0.048566 :`A` 1.0) 5.0))

(event `SetCamLocation`
  (params (Location :type "Vector Structure"))
  ;[1 1 1] Set Initial Cam spot
  (`SceneComponent.K2_SetWorldLocation` (`self.Camera`) (`KismetMathLibrary.MakeVector` Location_X Location_Y 200.0) false false))

(event `Key|Three`
  (params (Key :type "Key Structure"))
  ;[1 1 1] Save masks and coins
  (:`Pressed`
    (bind _asbp_game_instance (cast `/Game/Blueprints/MainGame/BP_GameInstance` (`GameplayStatics.GetGameInstance`)))
    (set `/Game/Blueprints/MainGame/BP_GameInstance.Masks` (`self.Masks`) _asbp_game_instance)
    (set `/Game/Blueprints/MainGame/BP_GameInstance.SavedCoins` (+ (`/Game/Blueprints/MainGame/BP_GameInstance.SavedCoins` _asbp_game_instance) (`self.Coins`)) _asbp_game_instance)
    (set `self.Coins` 0)))

(event `self.ReceiveTick`
  (params (DeltaSeconds :type "Float (single-precision)"))
  (bind _box (`self.Box`))
  (bind (_returnvalue_x _returnvalue_y) (`KismetMathLibrary.BreakVector` (`SceneComponent.K2_GetComponentLocation` _box)))
  (bind _worldlocation (`PlayerController.DeprojectMousePositionToWorld` (`GameplayStatics.GetPlayerController` 0)))
  ;[1 1 1] Attack Direction
  (`SceneComponent.K2_SetWorldRotation` _box (`KismetMathLibrary.FindLookAtRotation` (`KismetMathLibrary.MakeVector` _returnvalue_x _returnvalue_y) (`KismetMathLibrary.MakeVector` (.x _worldlocation) (.y _worldlocation))) false false))

(event `PickupSpeed`
  (bind _bpc_combat (`self.BPC_Combat`))
  (bind _charactermovement (`self.CharacterMovement`))
  (bind (_stats_health _stats_maxhealth _stats_damage _stats_speed _stats_attacksize) (break `/Game/Blueprints/MainGame/Combat/ST_Stats` (`/Game/Blueprints/MainGame/Combat/BPC_Combat.Stats` _bpc_combat)))
  (bind _returnvalue (+ _stats_speed 200.0))
  ;[1 1 1] Pickup Speed Item
  (set `/Game/Blueprints/MainGame/Combat/BPC_Combat.Stats` (make `/Game/Blueprints/MainGame/Combat/ST_Stats` _stats_health _stats_maxhealth _stats_damage _returnvalue _stats_attacksize) _bpc_combat)
  (set `CharacterMovementComponent.MaxWalkSpeed` _returnvalue _charactermovement)
  (set `CharacterMovementComponent.MaxAcceleration` (* _returnvalue 3.5) _charactermovement))

(event `Key|One`
  (params (Key :type "Key Structure"))
  ;[1 1 1] Force Coins and Masks
  (:`Pressed`
    (bind _result (`/Engine/EditorBlueprintResources/StandardMacros.IncrementInt` (`self.Masks`))
      (:`  `
        (bind _output_get (set `self.Masks` _result))
        (`KismetSystemLibrary.PrintString` (`KismetStringLibrary.Concat_StrStr` "Masks:" (`KismetStringLibrary.Conv_IntToString` _output_get)))))))

(event `Key|Two`
  (params (Key :type "Key Structure"))
  ;[1 1 1] Force Coins and Masks
  (:`Pressed`
    (bind _result (`/Engine/EditorBlueprintResources/StandardMacros.IncrementInt` (`self.Coins`))
      (:`  `
        (bind _output_get (set `self.Coins` _result))
        (`KismetSystemLibrary.PrintString` (`KismetStringLibrary.Concat_StrStr` "Coins:" (`KismetStringLibrary.Conv_IntToString` _output_get)))))))

(event `Key|LeftMouseButton`
  (params (Key :type "Key Structure"))
  (bind _cube (`self.Cube`))
  (bind _returnvalue (`SceneComponent.K2_GetComponentLocation` _cube))
  (bind (_stats_health _stats_maxhealth _stats_damage) (break `/Game/Blueprints/MainGame/Combat/ST_Stats` (`/Game/Blueprints/MainGame/Combat/BPC_Combat.Stats` (`self.BPC_Combat`))))
  ;[1 1 1] Attack
  (:`Pressed`
    (bind (_outhit _returnvalue_2) (`KismetSystemLibrary.SphereTraceSingleForObjects` :`Start` _returnvalue :`End` (+ _returnvalue (* (`SceneComponent.GetForwardVector` _cube) (`self.AttackSize`))) :`Radius` 100.0 :`ObjectTypes` (`|MakeArray` "ObjectTypeQuery3" :!type "EObjectTypeQuery Enum") :`bTraceComplex` true :`DrawDebugType` "ForDuration" :`DrawTime` 0.2))
    (if _returnvalue_2
      (`KismetSystemLibrary.PrintString` "Attacked")
      (message `/Game/Blueprints/MainGame/Combat/BP_Combat.TakeDamage` (`.HitActor` (`GameplayStatics.BreakHitResult` _outhit)) _stats_damage))))

(event `Key|Four`
  (params (Key :type "Key Structure"))
  (:`Pressed`
    (`GameplayStatics.OpenLevelBySoftObjectPtr` "/Game/Maps/MainArea.MainArea")))

(event `Death`
  (set `/Game/Blueprints/MainGame/Combat/BPC_Combat.IsInvincible` true (`self.BPC_Combat`))
  (`KismetSystemLibrary.PrintString` "Die")
  (`GameplayStatics.OpenLevelBySoftObjectPtr` "/Game/Maps/MainArea.MainArea"))

(event `Key|R`
  (params (Key :type "Key Structure"))
  (bind (_stats_health _stats_maxhealth _stats_damage _stats_speed _stats_attacksize) (break `/Game/Blueprints/MainGame/Combat/ST_Stats` (`/Game/Blueprints/MainGame/Combat/BPC_Combat.Stats` (`self.BPC_Combat`))))
  (:`Pressed`
    (`KismetSystemLibrary.PrintString` (`KismetStringLibrary.Concat_StrStr` "Health: " (`KismetStringLibrary.Conv_IntToString` _stats_health)) true true (struct :`R` 0.447917 :`B` 0.048566 :`A` 1.0) 5.0)))

(event `Key|T`
  (params (Key :type "Key Structure"))
  (bind _bpc_combat (`self.BPC_Combat`))
  (bind (_stats_health _stats_maxhealth _stats_damage _stats_speed _stats_attacksize) (break `/Game/Blueprints/MainGame/Combat/ST_Stats` (`/Game/Blueprints/MainGame/Combat/BPC_Combat.Stats` _bpc_combat)))
  (:`Pressed`
    (set `/Game/Blueprints/MainGame/Combat/BPC_Combat.Stats` (make `/Game/Blueprints/MainGame/Combat/ST_Stats` 100 _stats_maxhealth _stats_damage _stats_speed _stats_attacksize) _bpc_combat)))

(event `Key|P`
  (params (Key :type "Key Structure"))
  ;[1 1 1] Debug Cam
  (:`Pressed`
    (bind _returnvalue (`|SpawnActorFromClass` "/Game/Blueprints/BP_DebugPawn.BP_DebugPawn_C" (`self.GetTransform`) "Undefined" "MultiplyWithRoot" null null))
    (`Controller.Possess` (`GameplayStatics.GetPlayerController` 0) _returnvalue)))

(event `Key|E`
  (params (Key :type "Key Structure"))
  ;[1 1 1] Interacions
  (:`Pressed`
    (for _array_element (`self.GetOverlappingActors` null)
      (if (`KismetSystemLibrary.DoesImplementInterface` _array_element "/Game/Blueprints/Platformer/BP_InteractInterface.BP_InteractInterface_C")
        (message `/Game/Blueprints/Platformer/BP_InteractInterface.Interact` _array_element)
        (break)))))

(fn `Heal`
  (params (Target :type "Actor Object Reference") (InHeal :type Integer))
  (returns (OutHeal :type Integer))
  (return InHeal))

(fn `TakeDamage`
  (params (InDamage :type Integer))
  (returns (WasDamaged :type Boolean))
  (bind _bpc_combat (`self.BPC_Combat`))
  (bind _stats_health (break `/Game/Blueprints/MainGame/Combat/ST_Stats` (`/Game/Blueprints/MainGame/Combat/BPC_Combat.Stats` _bpc_combat)))
  (bind _damaged (`/Game/Blueprints/MainGame/Combat/BPC_Combat.TakeDamage` _bpc_combat InDamage))
  (`KismetSystemLibrary.PrintString` (`KismetStringLibrary.Concat_StrStr` "Health: " (`KismetStringLibrary.Conv_IntToString` _stats_health)))
  (return _damaged))

(fn `UserConstructionScript`
  (bind _bpc_combat (`self.BPC_Combat`))
  (`|ExecutionSequence`
    (:`then_0`
      (add `/Game/Blueprints/MainGame/Combat/BPC_Combat.Death` _bpc_combat (`|CreateDelegate` :!event `Death`))
      (add `/Game/Blueprints/MainGame/Combat/BPC_Combat.DamageResponse` _bpc_combat (`|CreateDelegate` :!event `DamageResponse`)))
    (:`then_1`
      (bind _asbp_game_instance (cast `/Game/Blueprints/MainGame/BP_GameInstance` (`GameplayStatics.GetGameInstance`)))
      (if (`/Game/Blueprints/MainGame/BP_GameInstance.Saved` _asbp_game_instance)
        (set `/Game/Blueprints/MainGame/Combat/BPC_Combat.Stats` (`/Game/Blueprints/MainGame/BP_GameInstance.Stats_GI` _asbp_game_instance) (`self.BPC_Combat`))))))