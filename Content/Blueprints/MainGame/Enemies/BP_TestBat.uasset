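; BP_TestBat is a test bat enemy that moves in circles, damages the player on contact and drops a coin on death.
; While alive, Tick adds a fixed yaw step and forward movement input, and capsule hits call TakeDamage on BP_Player using the bat's damage stat.
; BPCCombat handles incoming damage, with its Death event bound in the construction script to spawn BP_Coin and destroy the bat.
; Heal and DamageResponse are stubs.
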(event `self.ReceiveTick`
  (params (DeltaSeconds :type "Float (single-precision)"))
  (bind (_returnvalue_roll _returnvalue_pitch _returnvalue_yaw) (`KismetMathLibrary.BreakRotator` (`self.K2_GetActorRotation`)))
  (if (not (`self.Dead`))
    (`self.K2_SetActorRotation` (`KismetMathLibrary.MakeRotator` 0.0 0.0 (+ _returnvalue_yaw 5.0)))
    (`self.AddMovementInput` (`self.GetActorForwardVector`))))

(event `self.CapsuleComponent.OnComponentHit`
  (params (HitComponent :type "PrimitiveComponent Object Reference") (OtherActor :type "Actor Object Reference") (OtherComp :type "PrimitiveComponent Object Reference") (NormalImpulse :type "Vector Structure") (Hit :type "HitResult Structure (by ref)"))
  (bind (_stats_health _stats_maxhealth _stats_damage) (break `/Game/Blueprints/MainGame/Combat/ST_Stats` (`/Game/Blueprints/MainGame/Combat/BPC_Combat.Stats` (`self.BPC_Combat`))))
  (bind _asbp_player (cast `/Game/Blueprints/MainGame/BP_Player` OtherActor))
  (`/Game/Blueprints/MainGame/Combat/BP_Combat.TakeDamage` _asbp_player _stats_damage)
  (`KismetSystemLibrary.PrintString` "Attacked Player"))

(event `Death`
  (bind _returnvalue_location (`KismetMathLibrary.BreakTransform` (`self.GetTransform`)))
  (set `self.Dead` true)
  (`|SpawnActorFromClass` "/Game/Blueprints/MainGame/Combat/EnemyDrops/BP_Coin.BP_Coin_C" (`KismetMathLibrary.MakeTransform` _returnvalue_location) "Undefined" "MultiplyWithRoot" null null)
  (`KismetSystemLibrary.Delay` 0.1)
  (`self.K2_DestroyActor`))

(event `DamageResponse`)

(fn `Heal`
  (params (Target :type "Actor Object Reference") (InHeal :type Integer))
  (returns (OutHeal :type Integer))
  (return 0))

(fn `TakeDamage`
  (params (InDamage :type Integer))
  (returns (WasDamaged :type Boolean))
  (bind _stats_health (break `/Game/Blueprints/MainGame/Combat/ST_Stats` (`/Game/Blueprints/MainGame/Combat/BPC_Combat.Stats` (`self.BPC_Combat`))))
  (`/Game/Blueprints/MainGame/Combat/BPC_Combat.TakeDamage` (`self.BPC_Combat`) InDamage)
  (`KismetSystemLibrary.PrintString` (`KismetStringLibrary.Concat_StrStr` "Bat Health: " (`KismetStringLibrary.Conv_IntToString` _stats_health)))
  (return false))

(fn `UserConstructionScript`
  (bind _bpc_combat (`self.BPC_Combat`))
  (add `/Game/Blueprints/MainGame/Combat/BPC_Combat.Death` _bpc_combat (`|CreateDelegate` :!event `Death`))
  (add `/Game/Blueprints/MainGame/Combat/BPC_Combat.DamageResponse` _bpc_combat (`|CreateDelegate` :!event `DamageResponse`)))