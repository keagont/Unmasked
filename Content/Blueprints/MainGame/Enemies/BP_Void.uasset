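; BP_Void is an enemy Blueprint that hooks into the shared BPCCombat component, with most of its behavior still empty.
; The construction script binds events to the component's death and damage-response notifications; the Death, DamageResponse and capsule hit handlers have no logic.
; TakeDamage forwards damage to BPCCombat and always returns false, while Heal is a stub that returns zero.
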(event `self.CapsuleComponent.OnComponentHit`
  (params (HitComponent :type "PrimitiveComponent Object Reference") (OtherActor :type "Actor Object Reference") (OtherComp :type "PrimitiveComponent Object Reference") (NormalImpulse :type "Vector Structure") (Hit :type "HitResult Structure (by ref)")))

(event `Death`)

(event `Damage Response`)

(fn `Heal`
  (params (Target :type "Actor Object Reference") (InHeal :type Integer))
  (returns (OutHeal :type Integer))
  (return 0))

(fn `TakeDamage`
  (params (InDamage :type Integer))
  (returns (WasDamaged :type Boolean))
  (`/Game/Blueprints/MainGame/Combat/BPC_Combat.TakeDamage` (`self.BPC_Combat`) InDamage)
  (return false))

(fn `UserConstructionScript`
  (bind _bpc_combat (`self.BPC_Combat`))
  (add `/Game/Blueprints/MainGame/Combat/BPC_Combat.Death` _bpc_combat (`|CreateDelegate` :!event `Death`))
  (add `/Game/Blueprints/MainGame/Combat/BPC_Combat.DamageResponse` _bpc_combat (`|CreateDelegate` :!event `Damage Response`)))