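; BP_Boss_Blob is a Paper2D blob boss enemy that damages the player on capsule contact and spawns an exit door when it dies.
; Incoming damage is forwarded to the BPCCombat component, whose death and damage-response events are bound in the construction script.
; Death spawns BP_ExitDoor at the sprite location saved on BeginPlay, then destroys the boss.
; Damage response only prints health, and Heal just returns its input.
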(event `self.ReceiveBeginPlay`
  ;[1 1 1] Set spawn location
  (`KismetSystemLibrary.PrintString` "Blob Spawn")
  (set `self.SpawnLoc` (`SceneComponent.K2_GetComponentToWorld` (`self.PaperSprite`))))

(event `GetDamaged`
  (bind (_stats_health _stats_maxhealth) (break `/Game/Blueprints/MainGame/Combat/ST_Stats` (`/Game/Blueprints/MainGame/Combat/BPC_Combat.Stats` (`self.BPC_Combat`))))
  ;[1 1 1] Take Damage
  (`KismetSystemLibrary.PrintString` (`KismetStringLibrary.Concat_StrStr` (`KismetStringLibrary.Conv_IntToString` _stats_health) "/" (`KismetStringLibrary.Conv_IntToString` _stats_maxhealth) " Health") true true (struct :`R` 0.050321 :`G` 0.546875 :`A` 1.0) 5.0))

(event `Die`
  (bind _spawnloc_location (`KismetMathLibrary.BreakTransform` (`self.SpawnLoc`)))
  ;[1 1 1] Death
  (`KismetSystemLibrary.PrintString` "I am die" true true (struct :`R` 0.546875 :`G` 0.015206 :`A` 1.0) 5.0)
  (`|SpawnActorFromClass` "/Game/Blueprints/MainGame/LevelGen/BP_ExitDoor.BP_ExitDoor_C" (`KismetMathLibrary.MakeTransform` _spawnloc_location) "Undefined" "MultiplyWithRoot" null null)
  (`self.K2_DestroyActor`))

(event `self.CapsuleComponent.OnComponentHit`
  (params (HitComponent :type "PrimitiveComponent Object Reference") (OtherActor :type "Actor Object Reference") (OtherComp :type "PrimitiveComponent Object Reference") (NormalImpulse :type "Vector Structure") (Hit :type "HitResult Structure (by ref)"))
  (bind _asbp_player (cast `/Game/Blueprints/MainGame/BP_Player` OtherActor))
  (`/Game/Blueprints/MainGame/Combat/BP_Combat.TakeDamage` _asbp_player 10))

(fn `Heal`
  (params (Target :type "Actor Object Reference") (InHeal :type Integer))
  (returns (OutHeal :type Integer))
  (return InHeal))

(fn `TakeDamage`
  (params (InDamage :type Integer))
  (returns (WasDamaged :type Boolean))
  (bind _damaged (`/Game/Blueprints/MainGame/Combat/BPC_Combat.TakeDamage` (`self.BPC_Combat`) InDamage))
  (return _damaged))

(fn `UserConstructionScript`
  (bind _bpc_combat (`self.BPC_Combat`))
  (add `/Game/Blueprints/MainGame/Combat/BPC_Combat.Death` _bpc_combat (`|CreateDelegate` :!event `Die`))
  (add `/Game/Blueprints/MainGame/Combat/BPC_Combat.DamageResponse` _bpc_combat (`|CreateDelegate` :!event `GetDamaged`)))