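; BPC_Combat is a combat component that handles damage and death for its owner through a Stats struct.
; TakeDamage rejects hits while IsInvincible is set, otherwise subtracts the damage from Health and returns whether the hit landed.
; Remaining health triggers CallDamageResponse, while zero or less sets IsDead and triggers CallDeath, with no clamping of Health.
; The event graph holds no active logic.
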(fn `TakeDamage`
  (params (Damage :type Integer))
  (returns (Damaged :type Boolean))
  (bind (_stats_health _stats_maxhealth _stats_damage _stats_speed _stats_attacksize) (break `/Game/Blueprints/MainGame/Combat/ST_Stats` (`self.Stats`)))
  (if (`self.IsInvincible`)
    (return false)
    (else
      (bind _output_get (set `self.Stats` (make `/Game/Blueprints/MainGame/Combat/ST_Stats` (- _stats_health Damage) _stats_maxhealth _stats_damage _stats_speed _stats_attacksize)))
      (if (> (break `/Game/Blueprints/MainGame/Combat/ST_Stats` _output_get) 0)
        (`self.DamageResponse`)
        (else
          (set `self.IsDead` true)
          (`self.Death`)))
      (return true))))